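; Player pawn for a physics-driven rolling ball that gathers collectables and restarts the level when damaged.
; Move axis inputs apply torque to the sphere while movement is allowed.
; BeginPlay creates the HUD widget and fades the camera in from black.
; Any damage asks BP_TopDownMan_GM to restart the level, gated by a DoOnce, and a simple function increments the collectable count.
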(event `self.ReceiveBeginPlay`
  ;[1 1 1] Create HUD
  (bind _returnvalue (`|CreateWidget` "/Game/Blueprints/UI/W_HUD.W_HUD_C"))
  (`UserWidget.AddToViewport` _returnvalue 0)
  ;[1 1 1] Fade in on start
  (`PlayerCameraManager.StartCameraFade` :`self` (`GameplayStatics.GetPlayerCameraManager` 0) :`FromAlpha` 1.0 :`Duration` 2.0))

(event `InputAxis|MoveForward`
  (params (AxisValue :type "Float (single-precision)"))
  ;[1 1 1] Roll Forwards/Backwards
  (if (`self.CanMove`)
    (`PrimitiveComponent.AddTorqueInRadians` (`self.Sphere1`) (`KismetMathLibrary.MakeVector` 0.0 (* AxisValue 3000000.0)) "None" false)))

(event `InputAxis|MoveRight`
  (params (AxisValue :type "Float (single-precision)"))
  ;[1 1 1] Roll Left/Right
  (if (`self.CanMove`)
    (`PrimitiveComponent.AddTorqueInRadians` (`self.Sphere1`) (`KismetMathLibrary.MakeVector` (* (* AxisValue 3000000.0) -1.0)) "None" false)))

(event `self.ReceiveAnyDamage`
  (params (Damage :type "Float (single-precision)") (DamageType :type "DamageType Object Reference") (InstigatedBy :type "Controller Object Reference") (DamageCauser :type "Actor Object Reference"))
  ;[1 1 1] On Any Damage
  (`/Engine/EditorBlueprintResources/StandardMacros.DoOnce` false
    (:`Completed`
      (bind _asbp_top_down_man_gm (cast `/Game/Blueprints/GameMode/BP_TopDownMan_GM` (`GameplayStatics.GetGameMode`)))
      (`/Game/Blueprints/GameMode/BP_TopDownMan_GM.Restart Level` _asbp_top_down_man_gm))))

(fn `Increase Collectable Count`
  (`/Engine/EditorBlueprintResources/StandardMacros.IncrementInt` (`self.Collectables`)))

(fn `UserConstructionScript`)