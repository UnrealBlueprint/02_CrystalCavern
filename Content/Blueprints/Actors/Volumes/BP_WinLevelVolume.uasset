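; BP_WinLevelVolume is a volume that completes the level when the player overlaps it and no BP_Crystal actors remain in the world.
; On overlap, an IsPlayer check filters the actor, then AnyCrystalsRemaining counts crystals with GetAllActorsOfClass.
; LoadNextLevel finds the current level name in the Levels array and opens the following entry, or quits the game on the last one.
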(event `self.ReceiveActorBeginOverlap`
  (params (OtherActor :type "Actor Object Reference"))
  (`/Game/Blueprints/Actors/Collectables/MacroLib_CrystalCavern.Is Player` OtherActor
    (:`Is Player`
      (if (not (`self.Any Crystals Remaining`))
        (`self.Load Next Level`)))))

(fn `Any Crystals Remaining`
  (returns (ReturnValue :type Boolean))
  (bind _outactors (`GameplayStatics.GetAllActorsOfClass` "/Game/Blueprints/Actors/Collectables/BP_Crystal.BP_Crystal_C"))
  (return (> (`KismetArrayLibrary.Array_Length` _outactors) 0)))

(fn `Load Next Level`
  (locals (`Current Level Name` :type Name :default "None"))
  (bind _levels (`self.Levels`))
  (bind _returnvalue (`KismetArrayLibrary.Array_Find` _levels (`local.Current Level Name`)))
  (bind _returnvalue_2 (`GameplayStatics.GetCurrentLevelName` true))
  (set `local.Current Level Name` (`KismetStringLibrary.Conv_StringToName` _returnvalue_2))
  (if (== (`KismetArrayLibrary.Array_LastIndex` _levels) _returnvalue)
    (`KismetSystemLibrary.QuitGame` null "Quit")
    (else
      (`GameplayStatics.OpenLevel` (`|GetArrayItem` (`self.Levels`) (+ _returnvalue 1))))))

(fn `UserConstructionScript`)