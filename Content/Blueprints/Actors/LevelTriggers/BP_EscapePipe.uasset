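; BP_EscapePipe is a level-exit trigger that glides the player up a pipe and completes the level.
; When a PhysicsPawn_BP overlaps its Capsule, it disables that pawn's movement, physics simulation and collision.
; A timeline then lerps the pawn from the pipe's own actor location to GlideEndPoint.
; When the timeline finishes, it calls CompleteLevel on the BP_TopDownMan_GM game mode.
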(event `self.Capsule.OnComponentBeginOverlap`
  (params (OverlappedComponent :type "PrimitiveComponent Object Reference") (OtherActor :type "Actor Object Reference") (OtherComp :type "PrimitiveComponent Object Reference") (OtherBodyIndex :type Integer) (bFromSweep :type Boolean) (SweepResult :type "HitResult Structure (by ref)"))
  (bind _asphysics_pawn_bp (cast `/Game/Blueprints/Pawns/PhysicsPawn_BP` OtherActor))
  (set `self.Player Physics Pawn` _asphysics_pawn_bp)
  (`self.Disable Player Movement`)
  (set `self.Initial Smooth Location` (`self.K2_GetActorLocation`))
  (bind (_direction _lerp) (`Timeline|End Level Smooth Player Timeline` :!via `PlayFromStart`)
    (:`Update`
      (`self.Smooth Player to End Point` _lerp))
    (:`Complete Level`
      (`self.Finish Level`))))

(fn `Disable Player Movement`
  (bind _player_physics_pawn (`self.Player Physics Pawn`))
  (set `/Game/Blueprints/Pawns/PhysicsPawn_BP.CanMove` false _player_physics_pawn)
  (`PrimitiveComponent.SetSimulatePhysics` (`/Game/Blueprints/Pawns/PhysicsPawn_BP.Sphere1` _player_physics_pawn) false)
  (`self.SetActorEnableCollision` _player_physics_pawn false))

(fn `Finish Level`
  (bind _asbp_top_down_man_gm (cast `/Game/Blueprints/GameMode/BP_TopDownMan_GM` (`GameplayStatics.GetGameMode`)))
  (`/Game/Blueprints/GameMode/BP_TopDownMan_GM.Complete Level` _asbp_top_down_man_gm))

(fn `Smooth Player to End Point`
  (params (Alpha :type "Float (double-precision)"))
  (`self.K2_SetActorLocation` (`self.Player Physics Pawn`) (`KismetMathLibrary.VLerp` (`self.Initial Smooth Location`) (`SceneComponent.K2_GetComponentLocation` (`self.Glide End point`)) Alpha) false false) ; Glide player up pipe
)

(fn `UserConstructionScript`)