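; BP_Pickup is a collectable actor that gets drawn into the player when their pawn overlaps it.
; The first overlap passes a DoOnce, stores the start location and plays a timeline that moves the pickup toward the player's live position while shrinking it and fading its point light.
; When the timeline finishes, it increments the collectable count on PhysicsPawn_BP and destroys itself.
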(event `self.ReceiveActorBeginOverlap`
  (params (OtherActor :type "Actor Object Reference"))
  (if (== OtherActor (`GameplayStatics.GetPlayerPawn` 0))
    ;[1 0 0] IMPORTANT
    (`/Engine/EditorBlueprintResources/StandardMacros.DoOnce` false
      (:`Completed`
        (set `self.Smooth Start Location` (`self.K2_GetActorLocation`))
        (bind (_direction _smooth) (`Timeline|Timeline_0` :!via `PlayFromStart`)
          (:`Update`
            (`self.K2_SetActorLocation` (`KismetMathLibrary.VLerp` (`self.Smooth Start Location`) (`self.K2_GetActorLocation` (`GameplayStatics.GetPlayerPawn` 0)) _smooth))
            (`self.SetActorScale3D` (`KismetMathLibrary.VLerp` (1.0 1.0 1.0) (0.0 0.0 0.0) _smooth))
            (`LightComponent.SetIntensity` (`self.PointLight`) (`KismetMathLibrary.Lerp` 7437.270996 0.0 _smooth)))
          (:`Finished`
            (switch `ETimelineDirection` _direction
              (:`Forward`
                (bind _asphysics_pawn_bp (cast `/Game/Blueprints/Pawns/PhysicsPawn_BP` (`GameplayStatics.GetPlayerPawn` 0)))
                (`/Game/Blueprints/Pawns/PhysicsPawn_BP.Increase Collectable Count` _asphysics_pawn_bp)
                (`self.K2_DestroyActor`)))))))))

(fn `UserConstructionScript`)